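; BPC_HealthAndDamage is an actor component in the enemy folder that tracks health and reports damage and death to its owner.
; On BeginPlay it binds to the owner's OnTakeAnyDamage, then subtracts incoming damage from current health, clamped between zero and the maximum.
; While health remains, it sends the owner a damage-taken message with the damage type; at zero, a DoOnce sends a single time-to-die message.
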(event `self.ReceiveBeginPlay`
  (bind _returnvalue (`self.GetOwner`))
  (set `self.Owner` _returnvalue)
  (add `Actor.OnTakeAnyDamage` _returnvalue (delegate `BPC_DamageUpdate`)))

(event `BPC_DamageUpdate`
  (params (DamagedActor :type "Actor Object Reference") (Damage :type "Float (double-precision)") (DamageType :type "DamageType Object Reference") (InstigatedBy :type "Controller Object Reference") (DamageCauser :type "Actor Object Reference"))
  (bind _owner (`self.Owner`))
  (bind _output_get (set `self.HealthCurrent` (`KismetMathLibrary.FClamp` (- (`self.HealthCurrent`) Damage) 0.0 (`self.HealthMax`))))
  (`/Engine/EditorBlueprintResources/StandardMacros.CompareFloat` _output_get
    (:`>`
      (message `/Game/DigiPen/01_Enemy/AI_BPI.DamageTaken` _owner DamageType))
    (:`==`
      (`/Engine/EditorBlueprintResources/StandardMacros.DoOnce` false :!label _label
        (:`Completed`
          (message `/Game/DigiPen/01_Enemy/AI_BPI.TimeToDie` _owner))))
    (:`<`
      (goto _label))))

(fn `DamageTaken`
  (params (DamageType :type "DamageType Object Reference")))