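; Floor switch that fires an ACTIVATED event when a player-controlled Character steps on it, with optional hiding in game.
; Overlap begin and end drive DoOnce nodes that turn a dynamic material green on entry and red on exit.
; A non-looping MultiGate calls ResetSwitch after the first on-off cycle, which either greys out a fire-once switch or re-arms both DoOnces.
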(event `self.ReceiveBeginPlay`
  (bind _floorswitch (`self.FloorSwitch`))
  ;[1 1 1] Floor Switch Init
  (bind _returnvalue (`PrimitiveComponent.CreateDynamicMaterialInstance` _floorswitch 0 (`PrimitiveComponent.GetMaterial` _floorswitch 0) "None"))
  (set `self.FloorSwitchMaterial` _returnvalue)
  (`self.FloorSwitch_RED`)
  ;[1 1 1] Hide Visibilty of Switch
  (if (`self.SetHiddenInGame`)
    (`SceneComponent.SetVisibility` (`self.FloorSwitch`) false false)))

(event `FloorSwitch_RED`
  ;[1 1 1] Floor Switch Change Color
  (`MaterialInstanceDynamic.SetVectorParameterValue` (`self.FloorSwitchMaterial`) "Color" (struct :`R` 1.0 :`A` 1.0)))

(event `FloorSwitch_GREEN`
  ;[1 1 1] Floor Switch Change Color
  (`MaterialInstanceDynamic.SetVectorParameterValue` (`self.FloorSwitchMaterial`) "Color" (struct :`G` 1.0 :`A` 1.0)))

(event `FloorSwitch_Grey`
  ;[1 1 1] Floor Switch Change Color
  (`MaterialInstanceDynamic.SetVectorParameterValue` (`self.FloorSwitchMaterial`) "Color" (struct :`R` 0.276042 :`G` 0.276042 :`B` 0.276042 :`A` 1.0)))

(event `ResetSwitch`
  ;[1 1 1] Reset Switch OR Turn it off?
  (if (`self.DoesSwitchOnlyFireOnce`)
    (`self.FloorSwitch_Grey`)
    (else
      (`|ExecutionSequence`
        (:`then_0`
          (goto _label :!via `Reset`))
        (:`then_1`
          (goto _label_3 :!via `Reset`))))))

(event `self.FloorSwitch.OnComponentBeginOverlap`
  (params (OverlappedComponent :type "PrimitiveComponent Object Reference") (OtherActor :type "Actor Object Reference") (OtherComp :type "PrimitiveComponent Object Reference") (OtherBodyIndex :type Integer) (bFromSweep :type Boolean) (SweepResult :type "HitResult Structure (by ref)"))
  ;[1 1 1] Floor Switch Detect Player
  (`self.Cast_to_PlayerCharacter` OtherActor
    (:`then`
      (`/Engine/EditorBlueprintResources/StandardMacros.DoOnce` false :!label _label
        (:`Completed`
          (`self.FloorSwitch_GREEN`)
          (`self.FloorSwitch_ACTIVATED`)
          ;[1 1 1] After Switch has Turned ON and OFF once, check for reset
          (`|MultiGate` false :!label _label_2
            (:`Out 1`
              (`self.ResetSwitch`))))))))

(event `self.FloorSwitch.OnComponentEndOverlap`
  (params (OverlappedComponent :type "PrimitiveComponent Object Reference") (OtherActor :type "Actor Object Reference") (OtherComp :type "PrimitiveComponent Object Reference") (OtherBodyIndex :type Integer))
  ;[1 1 1] Floor Switch Detect Player
  (`self.Cast_to_PlayerCharacter` OtherActor
    (:`then`
      (`/Engine/EditorBlueprintResources/StandardMacros.DoOnce` false :!label _label_3
        (:`Completed`
          (`self.FloorSwitch_RED`)
          (goto _label_2))))))

(fn `UserConstructionScript`)