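; Four-panel door that opens when a player-controlled character enters its trigger and closes when they leave, gated by a forcefield.
; A timeline lerps each panel between start and end markers, playing forward to open and reversing to close.
; Any damage drops the forcefield, opening the door if the player is waiting, and leaving the trigger restores it, unless TurnOffForcefieldTrigger disables both.
; Flags set the initial door and forcefield states.
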(event `self.ReceiveBeginPlay`
  (bind _door_open_close (`self.Door Open/Close`))
  ;[1 1 1] Initialization
  (`|ExecutionSequence`
    (:`then_0`
      (if (not (`self.IsForcefieldActivated`))
        (`self.ForceField_DEACTIVATE`)))
    (:`then_1`
      (if (not (`self.IsDoorClosed`))
        (`self.Door_OPEN`)
        (`TimelineComponent.SetPlaybackPosition` _door_open_close (`TimelineComponent.GetTimelineLength` _door_open_close) false true)))))

(event `Door_OPEN`
  ;[1 1 1] Doors Open and Close
  (if (not (`self.NoDoor`))
    (bind (_direction _0_to_1) (`Timeline|Door Open/Close` :!label _label)
      (:`Update`
        (`SceneComponent.K2_SetWorldLocation` (`self.DoorUL`) (`KismetMathLibrary.VLerp` (`SceneComponent.K2_GetComponentLocation` (`self.ULStart`)) (`SceneComponent.K2_GetComponentLocation` (`self.ULEnd`)) _0_to_1) false false)
        (`SceneComponent.K2_SetWorldLocation` (`self.DoorUR`) (`KismetMathLibrary.VLerp` (`SceneComponent.K2_GetComponentLocation` (`self.URStart`)) (`SceneComponent.K2_GetComponentLocation` (`self.UREnd`)) _0_to_1) false false)
        (`SceneComponent.K2_SetWorldLocation` (`self.DoorLL`) (`KismetMathLibrary.VLerp` (`SceneComponent.K2_GetComponentLocation` (`self.LLStart`)) (`SceneComponent.K2_GetComponentLocation` (`self.LLEnd`)) _0_to_1) false false)
        (`SceneComponent.K2_SetWorldLocation` (`self.DoorLR`) (`KismetMathLibrary.VLerp` (`SceneComponent.K2_GetComponentLocation` (`self.LRStart`)) (`SceneComponent.K2_GetComponentLocation` (`self.LREnd`)) _0_to_1) false false)))))

(event `self.TriggerBox.OnComponentBeginOverlap`
  (params (OverlappedComponent :type "PrimitiveComponent Object Reference") (OtherActor :type "Actor Object Reference") (OtherComp :type "PrimitiveComponent Object Reference") (OtherBodyIndex :type Integer) (bFromSweep :type Boolean) (SweepResult :type "HitResult Structure (by ref)"))
  ;[1 1 1] Player in Trigger
  (`self.Cast_to_Player_Character` OtherActor
    (:`then`
      (set `self.IsPlayerInTrigger` true)
      (if (not (`self.IsForcefieldActivated`))
        (`self.Door_OPEN`)))))

(event `Door_CLOSE`
  ;[1 1 1] Doors Open and Close
  (if (not (`self.NoDoor`))
    (goto _label :!via `Reverse`)))

(event `self.TriggerBox.OnComponentEndOverlap`
  (params (OverlappedComponent :type "PrimitiveComponent Object Reference") (OtherActor :type "Actor Object Reference") (OtherComp :type "PrimitiveComponent Object Reference") (OtherBodyIndex :type Integer))
  ;[1 1 1] Player in Trigger
  (`self.Cast_to_Player_Character` OtherActor
    (:`then`
      (set `self.IsPlayerInTrigger` false)
      (`self.Door_CLOSE`)
      (if (not (`self.TurnOffForcefieldTrigger`))
        (`self.ForceField_ACTIVATE`)))))

(event `self.ReceiveAnyDamage`
  (params (Damage :type "Float (single-precision)") (DamageType :type "DamageType Object Reference") (InstigatedBy :type "Controller Object Reference") (DamageCauser :type "Actor Object Reference"))
  ;[1 1 1] Forcefield Detect Hit
  (if (not (`self.TurnOffForcefieldTrigger`))
    (`self.ForceField_DEACTIVATE`)))

(event `ForceField_DEACTIVATE`
  (bind _forcefield (`self.Forcefield`))
  ;[1 1 1] Forcefield Activate / Deactivate
  (`SceneComponent.SetVisibility` _forcefield false false)
  (`PrimitiveComponent.SetCollisionEnabled` _forcefield "NoCollision")
  (set `self.IsForcefieldActivated` false)
  (if (`self.IsPlayerInTrigger`)
    (`KismetSystemLibrary.Delay` 0.2)
    (`self.Door_OPEN`)))

(event `ForceField_ACTIVATE`
  (bind _forcefield (`self.Forcefield`))
  ;[1 1 1] Forcefield Activate / Deactivate
  (`SceneComponent.SetVisibility` _forcefield true false)
  (`PrimitiveComponent.SetCollisionEnabled` _forcefield "QueryAndPhysics")
  (set `self.IsForcefieldActivated` true))

(fn `UserConstructionScript`)