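; BP_SiTDoor is a hinged door that swings open when a player-controlled character enters its trigger volume and closes when they leave.
; BeginPlay derives the open rotation by yawing the hinge's world rotation a quarter turn, scaled by DoorOpenDirection.
; A timeline lerps between closed and open rotations, playing on overlap and reversing on exit.
; The construction script disables trigger collision when IsDoorActive is false.
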(event `self.ReceiveBeginPlay`
  (bind _output_get (set `self.HingeStartRotation` (`SceneComponent.K2_GetComponentRotation` (`self.Hinge`))))
  (set `self.HingeEndRotation` (`KismetMathLibrary.MakeRotator` (.roll _output_get) (.pitch _output_get) (+ (.yaw _output_get) (* (`self.DoorOpenDirection`) 90.0)))))

(event `self.TriggerVolume.OnComponentBeginOverlap`
  (params (OverlappedComponent :type "PrimitiveComponent Object Reference") (OtherActor :type "Actor Object Reference") (OtherComp :type "PrimitiveComponent Object Reference") (OtherBodyIndex :type Integer) (bFromSweep :type Boolean) (SweepResult :type "HitResult Structure (by ref)"))
  (bind _ascharacter (cast `Character` OtherActor))
  (cast `PlayerController` (`Pawn.GetController` _ascharacter))
  (bind (_direction _0_to_1_over_2sec) (`Timeline|Timeline-DoorOpen` :!label _label)
    (:`Update`
      (`SceneComponent.K2_SetWorldRotation` (`self.Hinge`) (`KismetMathLibrary.RLerp` (`self.HingeStartRotation`) (`self.HingeEndRotation`) _0_to_1_over_2sec) false false))))

(event `self.TriggerVolume.OnComponentEndOverlap`
  (params (OverlappedComponent :type "PrimitiveComponent Object Reference") (OtherActor :type "Actor Object Reference") (OtherComp :type "PrimitiveComponent Object Reference") (OtherBodyIndex :type Integer))
  (bind _ascharacter (cast `Character` OtherActor))
  (cast `PlayerController` (`Pawn.GetController` _ascharacter))
  (goto _label :!via `Reverse`))

(fn `UserConstructionScript`
  (if (not (`self.IsDoorActive`))
    (`PrimitiveComponent.SetCollisionEnabled` (`self.TriggerVolume`) "NoCollision")))