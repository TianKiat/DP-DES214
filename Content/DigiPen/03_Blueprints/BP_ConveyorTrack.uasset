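; Conveyor track actor that carries an anchor point along a straight path of configurable length.
; The construction script places the end position along local X, scales the track length component relative to its base length, and applies the timeline play rate.
; The StartConveyor event plays the MoveConveyor timeline from the start, lerping the anchor between the start and end world positions.
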(event `self.ReceiveBeginPlay`)

(event `StartConveyor`
  (bind (_direction _0_to_1) (`Timeline|MoveConveyor` :!via `PlayFromStart`)
    (:`Update`
      (`SceneComponent.K2_SetWorldLocation` (`self.AnchorPoint`) (`KismetMathLibrary.VLerp` (`SceneComponent.K2_GetComponentLocation` (`self.StartPosition`)) (`SceneComponent.K2_GetComponentLocation` (`self.EndPosition`)) _0_to_1) false false))))

(fn `UserConstructionScript`
  (`SceneComponent.K2_SetRelativeLocation` (`self.EndPosition`) (`KismetMathLibrary.MakeVector` (`self.LengthOfTrack`)) false false)
  (`SceneComponent.SetRelativeScale3D` (`self.TrackLength`) (`KismetMathLibrary.MakeVector` (/ (`self.LengthOfTrack`) (`self.BaseTrackLength`)) 1.0 1.0))
  (`TimelineComponent.SetPlayRate` (`self.MoveConveyor`) (`self.PlayRate`)))