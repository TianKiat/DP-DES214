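; Enemy turret that tracks and shoots at the player while they are inside its trigger volume.
; Tick rotates the weapon toward the player at constant speed and fires projectiles through a DoOnce and Delay cooldown, or resets the rotation when the player leaves.
; Damage and death events spawn explosion effects; death also adds fire, hides the trigger and weapon meshes, and stops tracking and firing.
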(event `self.ReceiveBeginPlay`
  (set `self.StartVector` (`SceneComponent.K2_GetComponentLocation` (`self.TurretWeaponParent`))))

(event `self.TriggerMesh.OnComponentBeginOverlap`
  (params (OverlappedComponent :type "PrimitiveComponent Object Reference") (OtherActor :type "Actor Object Reference") (OtherComp :type "PrimitiveComponent Object Reference") (OtherBodyIndex :type Integer) (bFromSweep :type Boolean) (SweepResult :type "HitResult Structure (by ref)"))
  (`self.Cast_to_PlayerCharacter` OtherActor)
  (set `self.IsPlayerInsideTrigger` true))

(event `self.ReceiveTick`
  (params (DeltaSeconds :type "Float (single-precision)"))
  (bind _turretweaponparent (`self.TurretWeaponParent`))
  (bind _turretweaponparent_2 (`self.TurretWeaponParent`))
  (set `self.DeltaTime` DeltaSeconds)
  (if (`self.IsDead?`)
    _
    (elif (`self.IsPlayerInsideTrigger`)
      ;[1 1 1] Rotate Turret to Follow Player
      (`SceneComponent.K2_SetWorldRotation` _turretweaponparent (`KismetMathLibrary.RInterpTo_Constant` (`SceneComponent.K2_GetComponentRotation` _turretweaponparent) (`KismetMathLibrary.FindLookAtRotation` (`SceneComponent.K2_GetComponentLocation` _turretweaponparent) (`self.K2_GetActorLocation` (`GameplayStatics.GetPlayerCharacter` 0))) (`self.DeltaTime`) 80.0) false false)
      (`self.Spawn_Projectile`)
      (else
        ;[1 1 1] Reset Rotation of the Turret
        (`SceneComponent.K2_SetWorldRotation` _turretweaponparent_2 (`KismetMathLibrary.RInterpTo_Constant` (`SceneComponent.K2_GetComponentRotation` _turretweaponparent_2) (`KismetMathLibrary.FindLookAtRotation` (`SceneComponent.K2_GetComponentLocation` _turretweaponparent_2) (`self.StartVector`)) (`self.DeltaTime`) 100.0) false false)))))

(event `self.TriggerMesh.OnComponentEndOverlap`
  (params (OverlappedComponent :type "PrimitiveComponent Object Reference") (OtherActor :type "Actor Object Reference") (OtherComp :type "PrimitiveComponent Object Reference") (OtherBodyIndex :type Integer))
  (`self.Cast_to_PlayerCharacter` OtherActor)
  (set `self.IsPlayerInsideTrigger` false))

(event `Spawn_Projectile`
  ;[1 1 1] Spawn Projectile at "ProjectileSpawnPoint"
  (`/Engine/EditorBlueprintResources/StandardMacros.DoOnce` false :!label _label
    (:`Completed`
      (`|SpawnActorFromClass` "/Game/DigiPen/02_Weapon/Projectile/Projectile_Child_Enemy.Projectile_Child_Enemy_C" (`SceneComponent.K2_GetComponentToWorld` (`self.ProjectileSpawnPoint`)) "Undefined" "OverrideRootScale" null null)
      (`KismetSystemLibrary.Delay` 1.0)
      (goto _label :!via `Reset`))))

(event `/Game/DigiPen/01_Enemy/AI_BPI.DamageTaken`
  (params (DamageType :type "DamageType Object Reference"))
  ;[1 1 1] Health and Damage
  (`GameplayStatics.SpawnEmitterAtLocation` "/Game/DigiPen/07_Particles/P_Explosion.P_Explosion" (`SceneComponent.K2_GetComponentLocation` (`self.TurretWeaponParent`)) (struct) (0.33 0.33 0.33)))

(event `/Game/DigiPen/01_Enemy/AI_BPI.TimeToDie`
  (bind _returnvalue (`SceneComponent.K2_GetComponentLocation` (`self.TurretWeaponParent`)))
  ;[1 1 1] Health and Damage
  (set `self.IsDead?` true)
  (`GameplayStatics.SpawnEmitterAtLocation` "/Game/DigiPen/07_Particles/P_Explosion.P_Explosion" _returnvalue (struct) (3.0 3.0 3.0))
  (`GameplayStatics.SpawnEmitterAtLocation` "/Game/DigiPen/07_Particles/P_Fire.P_Fire" _returnvalue)
  (`SceneComponent.SetVisibility` (`self.TriggerMesh`) false false)
  (`SceneComponent.SetVisibility` (`self.TurretWeapon`) false false))

(fn `UserConstructionScript`)