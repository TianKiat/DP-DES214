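; BP_VaultDoor is a two-leaf vault door that opens when all four of its locks are unlocked.
; Each lock update event stores its state, swaps that lock's light material on both gate sides, then rechecks all four.
; A timeline lerps the left and right doors open and reverses to close them if reclosing is allowed.
; Otherwise, the first full unlock latches the locks permanently open, ignoring later updates.
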(event `self.ReceiveBeginPlay`
  ;[1 1 1] ON Begin
  (`self.Init_All_Locks`))

(event `Init_All_Locks`
  ;[1 1 1] Initialize All Locks
  (`self.Update_Lock1` false)
  (`self.Update_Lock2` false)
  (`self.Update_Lock3` false)
  (`self.Update_Lock4` false))

(event `Update_Lock1`
  (params (bIsOpen :type Boolean :default false))
  ;[1 1 1] Update Locks
  (if (not (`self.bLocksPermanentlyOpened`))
    (bind _output_get (set `self.bLock1_IsOpen` bIsOpen))
    (if _output_get
      (set `self.Light_Color_To_Use` (`self.Light_UNLOCKED`))
      (else
        (set `self.Light_Color_To_Use` (`self.Light_LOCKED`))))
    (`PrimitiveComponent.SetMaterial` (`self.Gate_SideA`) 5 (`self.Light_Color_To_Use`))
    (`PrimitiveComponent.SetMaterial` (`self.Gate_SideB`) 5 (`self.Light_Color_To_Use`))
    (`self.Try_To_Open_Vault` :!label _label)))

(event `Try_To_Open_Vault`
  ;[1 1 1] Test All 4 Locks Are Unlocked
  (if (and (`self.bLock1_IsOpen`) (`self.bLock2_IsOpen`) (`self.bLock3_IsOpen`) (`self.bLock4_IsOpen`))
    (`self.Open_Vault_Doors`)
    (set `self.bDoorsOpening` true)
    (if (not (`self.bCanDoorsBeReclosed?`))
      (set `self.bLocksPermanentlyOpened` true))
    (elif (`self.bCanDoorsBeReclosed?`)
      (`self.Close_Vault_Doors`)
      (set `self.bDoorsOpening` false))))

(event `Update_Lock2`
  (params (bIsOpen :type Boolean :default false))
  ;[1 1 1] Update Locks
  (if (not (`self.bLocksPermanentlyOpened`))
    (bind _output_get (set `self.bLock2_IsOpen` bIsOpen))
    (if _output_get
      (set `self.Light_Color_To_Use` (`self.Light_UNLOCKED`))
      (else
        (set `self.Light_Color_To_Use` (`self.Light_LOCKED`))))
    (`PrimitiveComponent.SetMaterial` (`self.Gate_SideA`) 2 (`self.Light_Color_To_Use`))
    (`PrimitiveComponent.SetMaterial` (`self.Gate_SideB`) 2 (`self.Light_Color_To_Use`))
    (goto _label)))

(event `Update_Lock3`
  (params (bIsOpen :type Boolean :default false))
  ;[1 1 1] Update Locks
  (if (not (`self.bLocksPermanentlyOpened`))
    (bind _output_get (set `self.bLock3_IsOpen` bIsOpen))
    (if _output_get
      (set `self.Light_Color_To_Use` (`self.Light_UNLOCKED`))
      (else
        (set `self.Light_Color_To_Use` (`self.Light_LOCKED`))))
    (`PrimitiveComponent.SetMaterial` (`self.Gate_SideA`) 3 (`self.Light_Color_To_Use`))
    (`PrimitiveComponent.SetMaterial` (`self.Gate_SideB`) 3 (`self.Light_Color_To_Use`))
    (goto _label)))

(event `Update_Lock4`
  (params (bIsOpen :type Boolean :default false))
  ;[1 1 1] Update Locks
  (if (not (`self.bLocksPermanentlyOpened`))
    (bind _output_get (set `self.bLock4_IsOpen` bIsOpen))
    (if _output_get
      (set `self.Light_Color_To_Use` (`self.Light_UNLOCKED`))
      (else
        (set `self.Light_Color_To_Use` (`self.Light_LOCKED`))))
    (`PrimitiveComponent.SetMaterial` (`self.Gate_SideA`) 4 (`self.Light_Color_To_Use`))
    (`PrimitiveComponent.SetMaterial` (`self.Gate_SideB`) 4 (`self.Light_Color_To_Use`))
    (goto _label)))

(event `Open_Vault_Doors`
  ;[1 1 1] Open / Close Vault Doors
  (bind (_direction _0_to_1) (`Timeline|VaultDoor_Open` :!label _label_2)
    (:`Update`
      (`SceneComponent.K2_SetRelativeLocation` (`self.Door_R`) (`KismetMathLibrary.VLerp` (`self.DoorR_Start`) (`self.DoorR_End`) _0_to_1) false false)
      (`SceneComponent.K2_SetRelativeLocation` (`self.Door_L`) (`KismetMathLibrary.VLerp` (`self.DoorL_Start`) (`self.DoorL_End`) _0_to_1) false false))))

(event `Close_Vault_Doors`
  ;[1 1 1] Open / Close Vault Doors
  (goto _label_2 :!via `Reverse`))

(fn `UserConstructionScript`)