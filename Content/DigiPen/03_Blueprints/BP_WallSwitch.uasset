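; BP_WallSwitch is a switch that toggles between on and off when it takes any damage.
; Each toggle swaps the switch mesh material to match the new state and broadcasts the SwitchHasBeenTriggered dispatcher with that state.
; A DoOnce gates the damage event and resets after each hit unless the switch is flagged as one-use only.
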(event `self.ReceiveAnyDamage`
  (params (Damage :type "Float (single-precision)") (DamageType :type "DamageType Object Reference") (InstigatedBy :type "Controller Object Reference") (DamageCauser :type "Actor Object Reference"))
  (`/Engine/EditorBlueprintResources/StandardMacros.DoOnce` false :!label _label
    (:`Completed`
      (`self.CheckForSingleUse`)
      (if (`self.IsSwitchON`)
        (`self.Switch_OFF`)
        (else
          (`self.Switch_ON`))))))

(event `CheckForSingleUse`
  (if (not (`self.IsSwitchOneUseOnly`))
    (goto _label :!via `Reset`)))

(event `Switch_OFF`
  (`PrimitiveComponent.SetMaterial` (`self.Switch_Mesh`) 0 (`self.Material_OFF`))
  (set `self.IsSwitchON` false)
  (`self.Dispatch_SwitchHasBeenTriggered` (`self.IsSwitchON`) :!label _label_2))

(event `Switch_ON`
  (`PrimitiveComponent.SetMaterial` (`self.Switch_Mesh`) 0 (`self.Material_ON`))
  (set `self.IsSwitchON` true)
  (goto _label_2))

(fn `UserConstructionScript`)