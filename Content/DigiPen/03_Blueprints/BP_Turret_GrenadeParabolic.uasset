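; Turret that lobs physics grenades at a player-controlled Character inside its detection trigger.
; Trigger overlaps set or clear the target and start or stop the Fire_Rate timeline, whose event track times each shot.
; Each shot spawns a TEST_Grenade at the spawner and sets its physics velocity from SuggestProjectileVelocityCustomArc, aimed at the target's current location with random spread for a parabolic arc.
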(event `self.DetectionTrigger.OnComponentBeginOverlap`
  (params (OverlappedComponent :type "PrimitiveComponent Object Reference") (OtherActor :type "Actor Object Reference") (OtherComp :type "PrimitiveComponent Object Reference") (OtherBodyIndex :type Integer) (bFromSweep :type Boolean) (SweepResult :type "HitResult Structure (by ref)"))
  ;[1 1 1] Detect Player
  (bind _ascharacter (cast `Character` OtherActor))
  (if (`Pawn.IsPlayerControlled` _ascharacter)
    (set `self.TargetCharacter` _ascharacter)
    (`self.Activate_Turret`)))

(event `self.DetectionTrigger.OnComponentEndOverlap`
  (params (OverlappedComponent :type "PrimitiveComponent Object Reference") (OtherActor :type "Actor Object Reference") (OtherComp :type "PrimitiveComponent Object Reference") (OtherBodyIndex :type Integer))
  ;[1 1 1] Detect Player
  (bind _ascharacter (cast `Character` OtherActor))
  (if (`Pawn.IsPlayerControlled` _ascharacter)
    (set `self.TargetCharacter` null)
    (`self.Deactivate_Turret`)))

(event `Activate_Turret`
  ;[1 1 1] Grenade Timing
  (`Timeline|Fire_Rate` :!via `PlayFromStart` :!label _label
    (:`Fire_Grenade`
      (`self.Fire_Grenade`))))

(event `Deactivate_Turret`
  ;[1 1 1] Grenade Timing
  (goto _label :!via `Stop`))

(event `Fire_Grenade`
  (bind _returnvalue (`KismetMathLibrary.RandomFloatInRange` -100.0 100.0))
  ;[1 1 1] Fire Grenade
  ;;[1 1 1] Get Parabolic Velocity
  (bind _outlaunchvelocity (`GameplayStatics.SuggestProjectileVelocity_CustomArc` (`SceneComponent.K2_GetComponentLocation` (`self.GrenadeSpawner`)) (+ (`self.K2_GetActorLocation` (`self.TargetCharacter`)) (`KismetMathLibrary.MakeVector` _returnvalue _returnvalue _returnvalue)) 0.0 0.25))
  (bind _returnvalue_2 (`|SpawnActorFromClass` "/Game/DigiPen/02_Weapon/Projectile/TEST_Grenade.TEST_Grenade_C" (`SceneComponent.K2_GetComponentToWorld` (`self.GrenadeSpawner`)) "Undefined" "OverrideRootScale" null null)) ; Spawn Grenade
  ;;[1 1 1] Set Grenade to Parabolic Velocity
  (`PrimitiveComponent.SetPhysicsLinearVelocity` (`/Game/DigiPen/02_Weapon/Projectile/TEST_Grenade.Grenade` _returnvalue_2) _outlaunchvelocity false "None"))

(fn `UserConstructionScript`)