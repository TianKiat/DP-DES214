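; BP_HealingStation is a pickup-style station that heals characters who step into its beam.
; Overlapping the HealingBeam checks for a Character tagged CAN_HEAL, then applies negative damage scaled by HealingValue and activates the PHeal effect.
; Tick continuously spins the green cross sign mesh.
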(event `self.ReceiveTick`
  (params (DeltaSeconds :type "Float (single-precision)"))
  ;[1 1 1] Rotate Sign
  (`SceneComponent.K2_AddLocalRotation` (`self.GreenCross_SM`) (struct :`Yaw` -1.0) false false))

(event `self.HealingBeam.OnComponentBeginOverlap`
  (params (OverlappedComponent :type "PrimitiveComponent Object Reference") (OtherActor :type "Actor Object Reference") (OtherComp :type "PrimitiveComponent Object Reference") (OtherBodyIndex :type Integer) (bFromSweep :type Boolean) (SweepResult :type "HitResult Structure (by ref)"))
  ;[1 1 1] Restore Full Health on Enter
  (bind _ascharacter (cast `Character` OtherActor))
  (if (`self.ActorHasTag` _ascharacter "CAN_HEAL")
    (`GameplayStatics.ApplyDamage` _ascharacter (* (`self.Healing_Value`) -1.0))
    (`ActorComponent.Activate` (`self.P_Heal`) false)))

(fn `UserConstructionScript`)