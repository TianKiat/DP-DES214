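; BP_Target is a pop-up shooting target, colored green as friend or red otherwise, that starts raised or lowered.
; Damage while raised spins it, cuts its glow and timeline-flips the frame down, then hides it and disables collision.
; It can rise again after a delay by reversing that timeline.
; Each state change fires a dispatcher; the construction script tints a dynamic material and point light.
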(event `self.ReceiveBeginPlay`
  (bind _raise_lower_target (`self.Raise/Lower Target`))
  ;[1 1 1] Setup on Begin Play
  (if (`self.bSTARTwithTargetUp?`)
    (set `self.bIsTargetUp?` true)
    (`self.Glow_ON`)
    (else
      (set `self.bIsTargetUp?` false)
      (`TimelineComponent.SetPlaybackPosition` _raise_lower_target (`TimelineComponent.GetTimelineLength` _raise_lower_target) false true)
      (`self.Hide_Self`)
      (`self.Self_DisableCollision`)
      (`self.Glow_OFF`))))

(event `self.ReceiveAnyDamage`
  (params (Damage :type "Float (single-precision)") (DamageType :type "DamageType Object Reference") (InstigatedBy :type "Controller Object Reference") (DamageCauser :type "Actor Object Reference"))
  ;[1 1 1] Detect Damage Taken
  (if (`self.bIsTargetUp?`)
    (`self.Target_DOWN`)))

(event `Target_DOWN`
  ;[1 1 1] Flip Target Up and Down
  (`self.Feedback_SpinTarget`)
  (set `self.bIsTargetUp?` false)
  (`self.Update_Dispatch`)
  (`KismetSystemLibrary.Delay` 0.2)
  (`self.Glow_OFF`)
  (bind (_direction _0_to__90) (`Timeline|Raise/Lower Target` :!via `PlayFromStart` :!label _label)
    (:`Update`
      (`SceneComponent.K2_SetRelativeRotation` (`self.Frame`) (`KismetMathLibrary.MakeRotator` 0.0 _0_to__90) false false))
    (:`Finished`
      (if (not (`self.bIsTargetUp?`))
        (`self.Hide_Self`)
        (`self.Self_DisableCollision`)
        (`self.Check_Target_Auto_Reset`)))))

(event `Target_UP`
  ;[1 1 1] Flip Target Up and Down
  (`self.UnHide_Self`)
  (`self.Self_EnableCollision`)
  (set `self.bIsTargetUp?` true)
  (`self.Update_Dispatch`)
  (`self.Glow_ON`)
  (goto _label :!via `ReverseFromEnd`))

(event `Update_Dispatch`
  ;[1 1 1] Dispatcher
  (`self.Dispatcher_TargetStateChanged` (`self.bIsThis_FRIEND`) self (`self.bIsTargetUp?`)))

(event `Check_Target_Auto_Reset`
  ;[1 1 1] Check Target AutoReset
  (`KismetSystemLibrary.Delay` (`self.DelayBeforeReset`))
  (if (`self.bResetTargetAfterShot?`)
    (`self.Target_UP`)))

(event `Feedback_SpinTarget`
  ;[1 1 1] Feedback: Spin Target When Shot
  (bind (_direction _0_to_720) (`Timeline|TargetHit_SPIN` :!via `PlayFromStart`)
    (:`Update`
      (`SceneComponent.K2_SetRelativeRotation` (`self.Target`) (`KismetMathLibrary.MakeRotator` 0.0 _0_to_720) false false))))

(event `Hide_Self`
  ;[1 1 1] Hide / Reveal Self
  (`self.SetActorHiddenInGame` self true))

(event `Self_EnableCollision`
  ;[1 1 1] Collision Enable / Disable
  (`self.SetActorEnableCollision` self true))

(event `Glow_OFF`
  ;[1 1 1] Feedback: Glow Control
  (`self.Light_OFF`)
  (`MaterialInstanceDynamic.SetScalarParameterValue` (`self.Target_Material`) "Emissive" 0.0))

(event `UnHide_Self`
  ;[1 1 1] Hide / Reveal Self
  (`self.SetActorHiddenInGame` self false))

(event `Self_DisableCollision`
  ;[1 1 1] Collision Enable / Disable
  (`self.SetActorEnableCollision` self false))

(event `Glow_ON`
  ;[1 1 1] Feedback: Glow Control
  (`self.Light_ON`)
  (`MaterialInstanceDynamic.SetScalarParameterValue` (`self.Target_Material`) "Emissive" (`self.EmissiveIntensity`)))

(event `Light_OFF`
  ;[1 1 1] Lights On / Off
  (`SceneComponent.SetHiddenInGame` (`self.PointLight`) true false))

(event `Light_ON`
  ;[1 1 1] Lights On / Off
  (`SceneComponent.SetHiddenInGame` (`self.PointLight`) false false))

(fn `UserConstructionScript`
  (bind _color_red (`self.Color_Red`))
  (bind _target (`self.Target`))
  (bind _color_green (`self.Color_Green`))
  ;[1 1 1] Initialize Dynamic Material
  (bind _returnvalue (`PrimitiveComponent.CreateDynamicMaterialInstance` _target 1 (`PrimitiveComponent.GetMaterial` _target 1) "None"))
  (set `self.Target_Material` _returnvalue)
  ;[1 1 1] Set Color of Target and Lights
  (if (`self.bIsThis_FRIEND`)
    (`MaterialInstanceDynamic.SetVectorParameterValue` (`self.Target_Material`) "Color" _color_green)
    (`LightComponent.SetLightColor` (`self.PointLight`) _color_green true)
    (set `self.EmissiveIntensity` 5.0)
    (else
      (`MaterialInstanceDynamic.SetVectorParameterValue` (`self.Target_Material`) "Color" _color_red)
      (`LightComponent.SetLightColor` (`self.PointLight`) _color_red true))))